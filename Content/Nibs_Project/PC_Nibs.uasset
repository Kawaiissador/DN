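; Player controller for Nibs that runs game startup, menus and level transitions.
; BeginPlay applies display settings, loads the town or debug backroom, caches character and HUD through timeout macros, and registers Enhanced Input contexts.
; Transition events load level instances behind a loading screen, teleport the pawn, and usually set respawn and unload other maps.
; Escape drives the 3D option book and swaps gameplay/menu mappings; the progression flag is saved and loaded.
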(event Custom|LevelTransition%20to%20Day1
  (bind _floor1playerbeginloc (Variables|Default|GetFloor1PlayerBeginLoc))
  ;[0.15 0.15 0.15 0.5] Level Transitions
  (Default|LoadingScreen (Variables|Default|GetAs%20HUD_Core_Nibs))
  (Utilities|FlowControl|Delay 1.0)
  (Utilities|Platform|CollectGarbage)
  (bind _returnvalue (Class|LevelStreamingDynamic|LoadLevelInstance "Floor1Level_Inst" "0, 0, 0" "0, 0, 0" "" 0 false))
  (Variables|Default|SetFloor1Level_Inst _returnvalue)
  (Transformation|SetActorLocation (Game|Player|GetPlayerPawn 0) _floor1playerbeginloc false true)
  (CallFunction|SetLevelRespawnPoint _floor1playerbeginloc)
  (Game|Player|SetViewTargetwithBlend (Game|GetPlayerController 0) (Game|Player|GetPlayerPawn 0) 0.0 "VTBlend_EaseInOut" 0.0 false)
  ;;[1 0.5 0 0.5] Should unload all other levels beside needed one
  (CallFunction|FUnloadAllMaps "NewEnumerator3")
  (Class|GameplayStatics|FlushLevelStreaming)
  (Development|PrintString "Fade IN")
  (Default|LoadingScreen (Variables|Default|GetAs%20HUD_Core_Nibs))
  (Utilities|FlowControl|Delay 1.0)
  (Development|PrintString "Fade OUT")
  (Default|ToggleLoading (Variables|Default|GetAs%20HUD_Core_Nibs)))

(event Custom|Open/Closed%20Animation%20Completed
  (Variables|Default|SetPausedAnimationPlaying? false))

(event Custom|ControllerModeInOptionBook_Event
  (params (NewParam :type Integer))
  ;[0.15 0.15 0.15 0.5] Option Book related
  (Variables|Default|SetJoyPadControlMapping%200-1 NewParam) ; we set the Joypad Control mode here since save DON4T work
)

(event Custom|TriggerLevelTranstion
  (params (Level%20To%20trigger :type E_LevelList%20Enum :default "NewEnumerator0"))
  ;[0.15 0.15 0.15 0.5] Level Transitions
  ;;[1 0.5 0 0.5] From Trigger
  (Development|PrintString (Utilities|String|EnumtoString Level%20To%20trigger) true true "(R=0.115527,G=1.000000,B=0.000000,A=1.000000)" 1e+02)
  (switch Utilities|FlowControl|Switch|SwitchonE_LevelList Level%20To%20trigger
    (:NewEnumerator3
      (CallFunction|LevelTransitiontoDay1))
    (:NewEnumerator4
      (CallFunction|LevelTransitiontoTown))
    (:NewEnumerator5
      (CallFunction|LevelTransitiontoTutorial))
    (:NewEnumerator6
      (CallFunction|TransitiontoBackroom))))

(event Custom|LevelTransition%20to%20town
  (bind _townplayerbeginloc (Variables|Default|GetTownPlayerBeginLoc))
  ;[0.15 0.15 0.15 0.5] Level Transitions
  (Default|LoadingScreen (Variables|Default|GetAs%20HUD_Core_Nibs))
  (Utilities|FlowControl|Delay 1.0)
  (Utilities|Platform|CollectGarbage)
  (bind _returnvalue (Class|LevelStreamingDynamic|LoadLevelInstance "NibbsTownLvl_Inst" "0, 0, 0" "0, 0, 0" "" 0 false))
  (Variables|Default|SetNibbsTownLevel _returnvalue)
  (Transformation|SetActorLocation (Game|Player|GetPlayerPawn 0) _townplayerbeginloc false true)
  (CallFunction|SetLevelRespawnPoint _townplayerbeginloc)
  (Game|Player|SetViewTargetwithBlend (Game|GetPlayerController 0) (Game|Player|GetPlayerPawn 0) 0.0 "VTBlend_EaseInOut" 0.0 false)
  ;;[1 0.5 0 0.5] Should unload all other levels beside needed one
  (CallFunction|FUnloadAllMaps "NewEnumerator4")
  (Class|GameplayStatics|FlushLevelStreaming)
  (Development|PrintString "Fade IN")
  (Default|LoadingScreen (Variables|Default|GetAs%20HUD_Core_Nibs))
  (Utilities|FlowControl|Delay 1.0)
  (Development|PrintString "Fade OUT")
  (Default|ToggleLoading (Variables|Default|GetAs%20HUD_Core_Nibs)))

(event Custom|Transition%20ToBackroom
  (bind _backroombeginloc_0 (Variables|Default|GetBackroomBeginLoc_0))
  ;[0.15 0.15 0.15 0.5] Level Transitions
  (Default|LoadingScreen (Variables|Default|GetAs%20HUD_Core_Nibs))
  (Utilities|FlowControl|Delay 1.0)
  (Utilities|Platform|CollectGarbage)
  (bind _returnvalue (Class|LevelStreamingDynamic|LoadLevelInstance "BackroomsLvl_Inst" "0, 0, 0" "0, 0, 0" "" 0 false))
  (Variables|Default|SetBackroomsLvl_Inst _returnvalue)
  (Transformation|SetActorLocation (Game|Player|GetPlayerPawn 0) _backroombeginloc_0 false true)
  (CallFunction|SetLevelRespawnPoint _backroombeginloc_0)
  (Game|Player|SetViewTargetwithBlend (Game|GetPlayerController 0) (Game|Player|GetPlayerPawn 0) 0.0 "VTBlend_EaseInOut" 0.0 false)
  ;;[1 0.5 0 0.5] Should unload all other levels beside needed one
  (CallFunction|FUnloadAllMaps "NewEnumerator6")
  (Class|GameplayStatics|FlushLevelStreaming)
  (Development|PrintString "Fade IN")
  (Default|LoadingScreen (Variables|Default|GetAs%20HUD_Core_Nibs))
  (Utilities|FlowControl|Delay 1.0)
  (Development|PrintString "Fade OUT")
  (Default|ToggleLoading (Variables|Default|GetAs%20HUD_Core_Nibs)))

(event Custom|CloseMenu_Event
  ;[0.15 0.15 0.15 0.5] Option Book related
  (Variables|Default|SetMainMenu? false)
  (if (not (Variables|Default|GetPausedAnimationPlaying?))
    (Variables|Default|SetPausedAnimationPlaying? true)
    (bind _outactors (Actor|GetAllActorsOfClasswithTag "/Game/Nibs_Project/Blueprint/Props/OptionBook/BP_OptionBook.BP_OptionBook_C" "OptionBook"))
    (Utilities|FlowControl|Sequence
      (:then_0
        (Utilities|FlowControl|DoOnce false
          (:Completed
            (EventDispatchers|AssignCloseMenu (Utilities|Array|Get(acopy) _outactors) (EventDispatchers|CreateEvent :!event Custom|CloseMenu_Event))
            (EventDispatchers|BindEventtoCallLevelTransition (Utilities|Array|Get(acopy) _outactors) (EventDispatchers|CreateEvent :!event Custom|Level%20Transition%20Logic))
            (EventDispatchers|AssignControllerModeinOptionBook (Utilities|Array|Get(acopy) _outactors) (delegate Custom|ControllerModeInOptionBook_Event)))))
      (:then_1
        (if (Variables|Default|GetMainMenu?)
          (Transformation|SetActorLocation (Utilities|Array|Get(acopy) _outactors) (Variables|Default|GetMainMenuBookLoc) false true)))
      (:then_2
        ;;[0.15 0.15 0.15 0.5] Target Is 3DMeshBook
        (Default|PressEscape (Utilities|Array|Get(acopy) _outactors) (Variables|Default|GetMainMenu?))
        ;;[0.15 0.15 0.15 0.5] Target Is HUD core
        (Default|PressEscape (Variables|Default|GetAs%20HUD_Core_Nibs) (UserInterface|GetUserWidgetObject (Variables|/Game/Nibs_Project/Blueprint/Props/OptionBook/BP_OptionBook.BP_OptionBook_C|GetBook%20Widget%20High (Utilities|Array|Get(acopy) _outactors))))
        (Class|BPIPersistence|RequestLoad(Message) (Game|GetGameInstance) self)
        (Utilities|FlowControl|FlipFlop
          (:A
            ;;[1 0.5 0 0.5] This remove and Add the mapping
            (CallFunction|FPausINMapping))
          (:B
            (Utilities|FlowControl|Delay 0.5)
            (CallFunction|FPausOutMapping)))))))

(event Custom|LevelTransition%20to%20Debug
  ;[0.15 0.15 0.15 0.5] Level Transitions
  (Default|LoadingScreen (Variables|Default|GetAs%20HUD_Core_Nibs))
  (Utilities|FlowControl|Delay 1.0)
  (Utilities|Platform|CollectGarbage)
  (bind _returnvalue (Class|LevelStreamingDynamic|LoadLevelInstance "NibsTestLevel" "0, 0, 0" "0, 0, 0" "" 0 false))
  (Variables|Default|SetNibsTestLevel _returnvalue)
  (Transformation|SetActorLocation (Game|Player|GetPlayerPawn 0) "0, 0, 0" false true)
  (Game|Player|SetViewTargetwithBlend (Game|GetPlayerController 0) (Game|Player|GetPlayerPawn 0) 0.0 "VTBlend_EaseInOut" 0.0 false)
  (Class|GameplayStatics|FlushLevelStreaming)
  (Default|LoadingScreen (Variables|Default|GetAs%20HUD_Core_Nibs))
  (Utilities|FlowControl|Delay 1.0)
  (Default|ToggleLoading (Variables|Default|GetAs%20HUD_Core_Nibs)))

(event Custom|CE_PC_UpdateStamina
  (Default|UpdateStamina (Variables|Default|GetAs%20HUD_Core_Nibs) (/ (Variables|/Game/Nibs_Project/Blueprint/Player_Character/Nibs/BP_NibbsCharacter.BP_NibbsCharacter_C|GetStamina (Variables|Default|GetAs%20BP%20Nibs%20Character)) 1e+02)))

(event Custom|MainMenu%20Book
  ;[0.15 0.15 0.15 0.5] Level Transitions
  (Variables|Default|SetMainMenu? true)
  (CallFunction|OpenfromMainMenu))

(event Custom|OpenFromMainMenu
  ;[0.15 0.15 0.15 0.5] Option Book related
  (Variables|Default|SetMainMenu? true)
  (if (not (Variables|Default|GetPausedAnimationPlaying?))
    (Variables|Default|SetPausedAnimationPlaying? true)
    (bind _outactors (Actor|GetAllActorsOfClasswithTag "/Game/Nibs_Project/Blueprint/Props/OptionBook/BP_OptionBook.BP_OptionBook_C" "OptionBook"))
    (Utilities|FlowControl|Sequence
      (:then_0
        (Utilities|FlowControl|DoOnce false
          (:Completed
            (EventDispatchers|AssignCloseMenu (Utilities|Array|Get(acopy) _outactors) (EventDispatchers|CreateEvent :!event Custom|CloseMenu_Event))
            (EventDispatchers|BindEventtoCallLevelTransition (Utilities|Array|Get(acopy) _outactors) (EventDispatchers|CreateEvent :!event Custom|Level%20Transition%20Logic))
            (EventDispatchers|AssignControllerModeinOptionBook (Utilities|Array|Get(acopy) _outactors) (delegate Custom|ControllerModeInOptionBook_Event)))))
      (:then_1
        (if (Variables|Default|GetMainMenu?)
          (Transformation|SetActorLocation (Utilities|Array|Get(acopy) _outactors) (Variables|Default|GetMainMenuBookLoc) false true)))
      (:then_2
        ;;[0.15 0.15 0.15 0.5] Target Is 3DMeshBook
        (Default|PressEscape (Utilities|Array|Get(acopy) _outactors) (Variables|Default|GetMainMenu?))
        ;;[0.15 0.15 0.15 0.5] Target Is HUD core
        (Default|PressEscape (Variables|Default|GetAs%20HUD_Core_Nibs) (UserInterface|GetUserWidgetObject (Variables|/Game/Nibs_Project/Blueprint/Props/OptionBook/BP_OptionBook.BP_OptionBook_C|GetBook%20Widget%20High (Utilities|Array|Get(acopy) _outactors))))
        (Class|BPIPersistence|RequestLoad(Message) (Game|GetGameInstance) self)
        (Utilities|FlowControl|FlipFlop
          (:A
            ;;[1 0.5 0 0.5] This remove and Add the mapping
            (CallFunction|FPausINMapping))
          (:B
            (Utilities|FlowControl|Delay 0.5)
            (CallFunction|FPausOutMapping)))))))

(event Custom|Level%20Transition%20Logic
  (bind _returnvalue (Game|GetPlayerController 0))
  (bind _returnvalue_2 (PlayerController|LocalPlayerSubsystems|GetEnhancedInputLocalPlayerSubsystem _returnvalue))
  ;[0.15 0.15 0.15 0.5] Level Transitions
  (Development|PrintString "Level Tran,sition")
  (switch int (Variables|Default|GetProgressionFlag%200-4)
    (:0
      (CallFunction|LevelTransitiontoTutorial)
      (Input|AddMappingContext _returnvalue_2 "/Game/Nibs_Project/Input/NibsInput/IM_NibsController.IM_NibsController" 0 "(bIgnoreAllPressedKeysUntilRelease=True,bForceImmediately=False,bNotifyUserSettings=False)")
      (Input|AddMappingContext _returnvalue_2 "/Game/Nibs_Project/Input/DebugInput/IM_Debug.IM_Debug" 3 "(bIgnoreAllPressedKeysUntilRelease=True,bForceImmediately=False,bNotifyUserSettings=False)")
      (Input|AddMappingContext _returnvalue_2 "/Game/Nibs_Project/Input/MenusInput/IM_ToggleMenu.IM_ToggleMenu" 1 "(bIgnoreAllPressedKeysUntilRelease=True,bForceImmediately=False,bNotifyUserSettings=False)")
      (switch int (Variables|Default|GetJoyPadControlMapping%200-1) ; 0 is combat, and 1 is Parkour
        (:Default
          (Input|AddMappingContext _returnvalue_2 "/Game/Nibs_Project/Input/NibsInput/IM_NibsControllerJoyCombat.IM_NibsControllerJoyCombat" 2 "(bIgnoreAllPressedKeysUntilRelease=True,bForceImmediately=False,bNotifyUserSettings=False)" :!label _label)
          (Input|RemoveMappingContext _returnvalue_2 "/Game/Nibs_Project/Input/NibsInput/IM_NibsControllerJoyParkour.IM_NibsControllerJoyParkour" "(bIgnoreAllPressedKeysUntilRelease=True,bForceImmediately=False,bNotifyUserSettings=False)"))
        (:0
          (goto _label))
        (:1
          (Input|AddMappingContext _returnvalue_2 "/Game/Nibs_Project/Input/NibsInput/IM_NibsControllerJoyParkour.IM_NibsControllerJoyParkour" 2 "(bIgnoreAllPressedKeysUntilRelease=True,bForceImmediately=False,bNotifyUserSettings=False)")
          (Input|RemoveMappingContext _returnvalue_2 "/Game/Nibs_Project/Input/NibsInput/IM_NibsControllerJoyCombat.IM_NibsControllerJoyCombat" "(bIgnoreAllPressedKeysUntilRelease=True,bForceImmediately=False,bNotifyUserSettings=False)"))))
    (:5
      (CallFunction|LevelTransitiontoDebug))))

(event Custom|LevelTransitionToTutorial
  (bind _tutorialplayerbeginloc (Variables|Default|GetTutorialPlayerBeginLoc))
  ;[0.15 0.15 0.15 0.5] Level Transitions
  (Default|LoadingScreen (Variables|Default|GetAs%20HUD_Core_Nibs))
  (Utilities|FlowControl|Delay 1.0)
  (Utilities|Platform|CollectGarbage)
  (bind _returnvalue (Class|LevelStreamingDynamic|LoadLevelInstance "TutorialLevel_Inst" (Variables|Default|GetTutorialLevel_Inst_LOC) "0, 0, 0" "" 0 false))
  (Variables|Default|SetTutorialLevel_Inst _returnvalue)
  (Transformation|SetActorLocation (Game|Player|GetPlayerPawn 0) _tutorialplayerbeginloc false true)
  (CallFunction|SetLevelRespawnPoint _tutorialplayerbeginloc)
  (Game|Player|SetViewTargetwithBlend (Game|GetPlayerController 0) (Game|Player|GetPlayerPawn 0) 0.0 "VTBlend_EaseInOut" 0.0 false)
  ;;[1 0.5 0 0.5] Should unload all other levels beside needed one
  (CallFunction|FUnloadAllMaps "NewEnumerator5")
  (Class|GameplayStatics|FlushLevelStreaming)
  (Default|LoadingScreen (Variables|Default|GetAs%20HUD_Core_Nibs))
  (Utilities|FlowControl|Delay 1.0)
  (Default|ToggleLoading (Variables|Default|GetAs%20HUD_Core_Nibs)))

(event Custom|QuitGame
  (bind _asgi_nibbs_game_instance (Utilities|Casting|CastToGI_NibbsGameInstance (Game|GetGameInstance)))
  (Class|BPIPersistence|RequestSave(Message) self false)
  (Default|SaveGame _asgi_nibbs_game_instance false)
  (Utilities|FlowControl|DelayUntilNextTick)
  (Game|QuitGame 0 "Quit" false))

(event Input|EnhancedActionEvents|EnhancedInputActionIA_GO-Back_Menu
  (params (ActionValue :type Boolean) (ElapsedSeconds :type Float%20%28double-precision%29) (TriggeredSeconds :type Float%20%28double-precision%29) (InputAction :type Input%20Action%20Object%20Reference :default "/Game/Nibs_Project/Input/MenusInput/IA_GO-Back_Menu.IA_GO-Back_Menu"))
  ;[0.15 0.15 0.15 0.5] Option Book related
  (:Completed
    (if (not (Variables|Default|GetPausedAnimationPlaying?))
      (bind _outactors (Actor|GetAllActorsOfClasswithTag "/Game/Nibs_Project/Blueprint/Props/OptionBook/BP_OptionBook.BP_OptionBook_C" "OptionBook"))
      (Default|GOBack (Utilities|Array|Get(acopy) _outactors)))))

(event Input|EnhancedActionEvents|EnhancedInputActionIA_Escape
  (params (ActionValue :type Boolean) (ElapsedSeconds :type Float%20%28double-precision%29) (TriggeredSeconds :type Float%20%28double-precision%29) (InputAction :type Input%20Action%20Object%20Reference :default "/Game/Nibs_Project/Input/MenusInput/IA_Escape.IA_Escape"))
  ;[0.15 0.15 0.15 0.5] Option Book related
  (:Completed
    (if (not (Variables|Default|GetPausedAnimationPlaying?))
      (Variables|Default|SetPausedAnimationPlaying? true)
      (bind _outactors (Actor|GetAllActorsOfClasswithTag "/Game/Nibs_Project/Blueprint/Props/OptionBook/BP_OptionBook.BP_OptionBook_C" "OptionBook"))
      (Utilities|FlowControl|Sequence
        (:then_0
          (Utilities|FlowControl|DoOnce false
            (:Completed
              (EventDispatchers|AssignCloseMenu (Utilities|Array|Get(acopy) _outactors) (EventDispatchers|CreateEvent :!event Custom|CloseMenu_Event))
              (EventDispatchers|BindEventtoCallLevelTransition (Utilities|Array|Get(acopy) _outactors) (EventDispatchers|CreateEvent :!event Custom|Level%20Transition%20Logic))
              (EventDispatchers|AssignControllerModeinOptionBook (Utilities|Array|Get(acopy) _outactors) (delegate Custom|ControllerModeInOptionBook_Event)))))
        (:then_1
          (if (Variables|Default|GetMainMenu?)
            (Transformation|SetActorLocation (Utilities|Array|Get(acopy) _outactors) (Variables|Default|GetMainMenuBookLoc) false true)))
        (:then_2
          ;;[0.15 0.15 0.15 0.5] Target Is 3DMeshBook
          (Default|PressEscape (Utilities|Array|Get(acopy) _outactors) (Variables|Default|GetMainMenu?))
          ;;[0.15 0.15 0.15 0.5] Target Is HUD core
          (Default|PressEscape (Variables|Default|GetAs%20HUD_Core_Nibs) (UserInterface|GetUserWidgetObject (Variables|/Game/Nibs_Project/Blueprint/Props/OptionBook/BP_OptionBook.BP_OptionBook_C|GetBook%20Widget%20High (Utilities|Array|Get(acopy) _outactors))))
          (Class|BPIPersistence|RequestLoad(Message) (Game|GetGameInstance) self)
          (Utilities|FlowControl|FlipFlop
            (:A
              ;;[1 0.5 0 0.5] This remove and Add the mapping
              (CallFunction|FPausINMapping))
            (:B
              (Utilities|FlowControl|Delay 0.5)
              (CallFunction|FPausOutMapping))))))))

(event Input|EnhancedActionEvents|EnhancedInputActionIA_DebugMenuToggle
  (params (ActionValue :type Boolean) (ElapsedSeconds :type Float%20%28double-precision%29) (TriggeredSeconds :type Float%20%28double-precision%29) (InputAction :type Input%20Action%20Object%20Reference :default "/Game/Nibs_Project/Input/DebugInput/IA_DebugMenuToggle.IA_DebugMenuToggle"))
  ;[0.15 0.15 0.15 0.5] We get the Input for toggling the DebugHUD, and send it to the Toggle DEbug event node inside the HUD blueprint
  (Default|ToggleDebugHud (Variables|Default|GetAs%20HUD_Core_Nibs)))

(event EventBeginPlay
  (bind _returnvalue (Game|GetPlayerController 0))
  (bind _returnvalue_2 (PlayerController|LocalPlayerSubsystems|GetEnhancedInputLocalPlayerSubsystem _returnvalue))
  (Utilities|FlowControl|Sequence
    (:then_0
      (bind _returnvalue_3 (Settings|GetGameUserSettings))
      (Class|GameUserSettings|SetFullscreenMode _returnvalue_3 "WindowedFullscreen")
      (Class|GameUserSettings|SetFrameRateLimit _returnvalue_3 6e+01)
      (Class|GameUserSettings|SetResolutionScaleValueEx _returnvalue_3 (Math|Conversions|ToFloat(Integer) (* (/ (.y (Variables|Default|GetDefaultScreenRes)) (.y (Class|GameUserSettings|GetDesktopResolution _returnvalue_3))) 100)))
      (Class|GameUserSettings|SetScreenResolution _returnvalue_3 (Variables|Default|GetDefaultScreenRes))
      (Class|GameUserSettings|ApplySettings _returnvalue_3 false))
    (:then_1
      (if (Variables|Default|GetDebugON?%20PC)
        (Utilities|FlowControl|Delay 1.0 :!label _label)
        (Utilities|FlowControl|Sequence
          (:then_0
            (bind _asbp_nibs_character (Utilities|GetBPNibsCharacter 1e+01)
              (:Success
                (bind _output_get (Variables|Default|SetAs%20BP%20Nibs%20Character _asbp_nibs_character))
                (EventDispatchers|BindEventtoUpdateStamina _output_get (EventDispatchers|CreateEvent :!event Custom|CE_PC_UpdateStamina)))
              (:Failed
                (Development|PrintText "BP_NibScharacter Failed To Cast After 10second Timeout" true true "(R=1.000000,G=0.918112,B=0.000000,A=1.000000)" 5e+01))))
          (:then_1
            ;[0.15 0.15 0.15 0.5] Basicly, cast to is kinda bad, so we want to limit it, so we Cast only once to the HUD_Core (here being nibs) Then promote that to a variable we can reuse, idk why its better honestly, but people say it is.
            ;
            ; And This is so we get the HUD inside the PlayerController so we can communicate between both
            ;
            ; Cast can also fail, wich could be bad, so i think i should either have a  printstring for every "can fail" type node or do the macro thingy that extend and loop to allow some retry
            ;
            ; We can use a MacroLibrary (wich is class specific idk what that means!, also FunctionLibrary are usefull too apparently
            ;;[0.15 0.15 0.15 0.5] This is a Macro that Loop for 10sec trying to cast until it succeed ot timeout
            (bind _as_hud_core_nibs (Utilities|GetHUDCoreNibs 1e+01)
              (:Success
                (bind _output_get_2 (Variables|Default|SetAs%20HUD_Core_Nibs _as_hud_core_nibs))
                (EventDispatchers|BindEventtoQuitGame _output_get_2 (delegate Custom|QuitGame)))
              (:Failed
                (Development|PrintText "HUD_Nibs Failed To Cast After 10second Timeout" true true "(R=0.000000,G=0.660000,B=1.000000,A=1.000000)" 1e+01))))
          (:then_2
            (Default|CEPCNibbsSuccessInitialize (Variables|Default|GetAs%20HUD_Core_Nibs))
            (CallFunction|FRegisterMappingContext))
          (:then_3
            (bind _outactors (Actor|GetAllActorsOfClasswithTag "/Game/Nibs_Project/Blueprint/Props/OptionBook/BP_OptionBook.BP_OptionBook_C" "OptionBook"))
            (EventDispatchers|BindEventtoOpen/CloseCompleted (Utilities|Array|Get(acopy) _outactors) (delegate Custom|Open/Closed%20Animation%20Completed)))
          (:then_4
            (if (Variables|Default|GetDebugON?%20PC)
              ;[0.15 0.15 0.15 0.5] put debug level to load here
              (CallFunction|TransitiontoBackroom)
              (Utilities|FlowControl|DoOnce false
                (:Completed
                  ;[0.15 0.15 0.15 0.5] Level Transitions
                  (Input|AddMappingContext _returnvalue_2 "/Game/Nibs_Project/Input/NibsInput/IM_NibsController.IM_NibsController" 0 "(bIgnoreAllPressedKeysUntilRelease=True,bForceImmediately=False,bNotifyUserSettings=False)")
                  (Input|AddMappingContext _returnvalue_2 "/Game/Nibs_Project/Input/DebugInput/IM_Debug.IM_Debug" 3 "(bIgnoreAllPressedKeysUntilRelease=True,bForceImmediately=False,bNotifyUserSettings=False)")
                  (Input|AddMappingContext _returnvalue_2 "/Game/Nibs_Project/Input/MenusInput/IM_ToggleMenu.IM_ToggleMenu" 1 "(bIgnoreAllPressedKeysUntilRelease=True,bForceImmediately=False,bNotifyUserSettings=False)")
                  (switch int (Variables|Default|GetJoyPadControlMapping%200-1) ; 0 is combat, and 1 is Parkour
                    (:Default
                      (Input|AddMappingContext _returnvalue_2 "/Game/Nibs_Project/Input/NibsInput/IM_NibsControllerJoyCombat.IM_NibsControllerJoyCombat" 2 "(bIgnoreAllPressedKeysUntilRelease=True,bForceImmediately=False,bNotifyUserSettings=False)" :!label _label_2)
                      (Input|RemoveMappingContext _returnvalue_2 "/Game/Nibs_Project/Input/NibsInput/IM_NibsControllerJoyParkour.IM_NibsControllerJoyParkour" "(bIgnoreAllPressedKeysUntilRelease=True,bForceImmediately=False,bNotifyUserSettings=False)"))
                    (:0
                      (goto _label_2))
                    (:1
                      (Input|AddMappingContext _returnvalue_2 "/Game/Nibs_Project/Input/NibsInput/IM_NibsControllerJoyParkour.IM_NibsControllerJoyParkour" 2 "(bIgnoreAllPressedKeysUntilRelease=True,bForceImmediately=False,bNotifyUserSettings=False)")
                      (Input|RemoveMappingContext _returnvalue_2 "/Game/Nibs_Project/Input/NibsInput/IM_NibsControllerJoyCombat.IM_NibsControllerJoyCombat" "(bIgnoreAllPressedKeysUntilRelease=True,bForceImmediately=False,bNotifyUserSettings=False)"))))))))
        (else
          ;[0.15 0.15 0.15 0.5] Load Title Screen (and in futur all basic stuff like character, lights. post process idk)
          (bind (_boutsuccess _returnvalue_4) (Class|LevelStreamingDynamic|LoadLevelInstance "NibbsTownLvl_Inst" "0, 0, 0" "0, 0, 0" "" 0 false))
          (if _boutsuccess
            (Variables|Default|SetNibbsTownLvl_Inst _returnvalue_4)
            (goto _label)
            (else
              (Development|PrintString "Failed to load level instant" true true "(R=0.000000,G=0.660000,B=1.000000,A=1.000000)" 1e+01))))))))

(event EventSaveData
  (params (SaveGameRef :type SG%20Nibbs%20Save%20Object%20Reference))
  (Variables|/Game/Nibs_Project/SG_NibbsSave.SG_NibbsSave_C|SetLevel%200-4 SaveGameRef (Variables|Default|GetProgressionFlag%200-4)))

(event EventLoadData
  (params (SaveGameRef :type SG%20Nibbs%20Save%20Object%20Reference))
  (Variables|Default|SetProgressionFlag%200-4 (Variables|/Game/Nibs_Project/SG_NibbsSave.SG_NibbsSave_C|GetLevel%200-4 SaveGameRef)))

(event EventTick
  (params (DeltaSeconds :type Float%20%28single-precision%29))
  (bind _progressionflag_0_4 (Variables|Default|GetProgressionFlag%200-4))
  (if (== _progressionflag_0_4 4)
    (Development|PrintString (Utilities|String|Append "Day : " "7") true true "(R=0.000000,G=0.660000,B=1.000000,A=1.000000)" 2.0 "Saved Level")
    (else
      (Development|PrintString (Utilities|String|Append "Day : " (Utilities|String|ToString(Integer) _progressionflag_0_4)) true true "(R=0.000000,G=0.660000,B=1.000000,A=1.000000)" 2.0 "Saved Level"))))

(event Input|KeyboardEvents|DebugKeyF
  (params (Key :type Key%20Structure :default "None") (ActionValue :type Input%20Action%20Value%20Structure)))

(event Input|KeyboardEvents|DebugKeyR
  (params (Key :type Key%20Structure :default "None") (ActionValue :type Input%20Action%20Value%20Structure))
  (bind _as_bp_nibs_character (Variables|Default|GetAs%20BP%20Nibs%20Character))
  (:Pressed
    (Transformation|SetActorLocation _as_bp_nibs_character (.SpawnLoc (Utilities|Struct|BreakS_Char_DefaultVariableInfo (Variables|/Game/Nibs_Project/Blueprint/Player_Character/Nibs/BP_NibbsCharacter.BP_NibbsCharacter_C|GetS_Char_DefaultVariables _as_bp_nibs_character))) false true)))

(event Input|KeyboardEvents|AnyKey
  (params (Key :type Key%20Structure :default "None"))
  (:Pressed
    (if (not (Variables|Default|GetDebugON?%20PC))
      (if (Widget|IsVisible (Variables|/Game/Nibs_Project/HUD_CORE_Nibs.HUD_CORE_Nibs_C|GetMainMenu (Variables|Default|GetAs%20HUD_Core_Nibs)))
        (Default|ToggleTittleScreen (Variables|Default|GetAs%20HUD_Core_Nibs))
        ;[0.15 0.15 0.15 0.5] We can plug any event we want here To transition from tittle screen
        (EventDispatchers|BindEventtoTitleScreenEnd (Variables|Default|GetAs%20HUD_Core_Nibs) (EventDispatchers|CreateEvent :!event Custom|MainMenu%20Book))))))

(fn ConstructionScript)

(fn FAddGameplayMappingContext
  (bind _returnvalue (Game|GetPlayerController 0))
  (bind _returnvalue_2 (PlayerController|LocalPlayerSubsystems|GetEnhancedInputLocalPlayerSubsystem _returnvalue))
  (Input|AddMappingContext _returnvalue_2 "/Game/Nibs_Project/Input/NibsInput/IM_NibsController.IM_NibsController" 0 "(bIgnoreAllPressedKeysUntilRelease=True,bForceImmediately=False,bNotifyUserSettings=False)")
  (Input|AddMappingContext _returnvalue_2 "/Game/Nibs_Project/Input/MenusInput/IM_ToggleMenu.IM_ToggleMenu" 1 "(bIgnoreAllPressedKeysUntilRelease=True,bForceImmediately=False,bNotifyUserSettings=False)"))

(fn FRemoveGameplayMappingContext
  (bind _returnvalue (Game|GetPlayerController 0))
  (bind _returnvalue_2 (PlayerController|LocalPlayerSubsystems|GetEnhancedInputLocalPlayerSubsystem _returnvalue))
  (Input|RemoveMappingContext _returnvalue_2 "/Game/Nibs_Project/Input/NibsInput/IM_NibsController.IM_NibsController" "(bIgnoreAllPressedKeysUntilRelease=True,bForceImmediately=False,bNotifyUserSettings=False)")
  (Input|RemoveMappingContext _returnvalue_2 "/Game/Nibs_Project/Input/MenusInput/IM_ToggleMenu.IM_ToggleMenu" "(bIgnoreAllPressedKeysUntilRelease=True,bForceImmediately=False,bNotifyUserSettings=False)"))

(fn FPausINMapping
  (bind _returnvalue (Game|GetPlayerController 0))
  (bind _returnvalue_2 (PlayerController|LocalPlayerSubsystems|GetEnhancedInputLocalPlayerSubsystem _returnvalue))
  (Input|RemoveMappingContext _returnvalue_2 "/Game/Nibs_Project/Input/NibsInput/IM_NibsController.IM_NibsController" "(bIgnoreAllPressedKeysUntilRelease=True,bForceImmediately=False,bNotifyUserSettings=False)")
  (Input|RemoveMappingContext _returnvalue_2 "/Game/Nibs_Project/Input/NibsInput/IM_NibsControllerJoyParkour.IM_NibsControllerJoyParkour" "(bIgnoreAllPressedKeysUntilRelease=True,bForceImmediately=False,bNotifyUserSettings=False)")
  (Input|RemoveMappingContext _returnvalue_2 "/Game/Nibs_Project/Input/NibsInput/IM_NibsControllerJoyCombat.IM_NibsControllerJoyCombat" "(bIgnoreAllPressedKeysUntilRelease=True,bForceImmediately=False,bNotifyUserSettings=False)")
  (Input|AddMappingContext _returnvalue_2 "/Game/Nibs_Project/Input/MenusInput/IM_MenuNavigation.IM_MenuNavigation" 3 "(bIgnoreAllPressedKeysUntilRelease=True,bForceImmediately=False,bNotifyUserSettings=False)"))

(fn FPausOutMapping
  (bind _returnvalue (Game|GetPlayerController 0))
  (bind _returnvalue_2 (PlayerController|LocalPlayerSubsystems|GetEnhancedInputLocalPlayerSubsystem _returnvalue))
  (Input|RemoveMappingContext _returnvalue_2 "/Game/Nibs_Project/Input/MenusInput/IM_MenuNavigation.IM_MenuNavigation" "(bIgnoreAllPressedKeysUntilRelease=True,bForceImmediately=False,bNotifyUserSettings=False)")
  (Input|AddMappingContext _returnvalue_2 "/Game/Nibs_Project/Input/NibsInput/IM_NibsController.IM_NibsController" 0 "(bIgnoreAllPressedKeysUntilRelease=True,bForceImmediately=False,bNotifyUserSettings=False)") ; This is keyboard
  (switch int (Variables|Default|GetJoyPadControlMapping%200-1) ; 0 is combat, and 1 is Parkour
    (:0
      (Input|AddMappingContext _returnvalue_2 "/Game/Nibs_Project/Input/NibsInput/IM_NibsControllerJoyCombat.IM_NibsControllerJoyCombat" 2 "(bIgnoreAllPressedKeysUntilRelease=True,bForceImmediately=False,bNotifyUserSettings=False)"))
    (:1
      (Input|AddMappingContext _returnvalue_2 "/Game/Nibs_Project/Input/NibsInput/IM_NibsControllerJoyParkour.IM_NibsControllerJoyParkour" 2 "(bIgnoreAllPressedKeysUntilRelease=True,bForceImmediately=False,bNotifyUserSettings=False)"))))

(fn SetLevelRespawnPoint
  (params (SpawnLoc :type Vector))
  (bind _as_bp_nibs_character (Variables|Default|GetAs%20BP%20Nibs%20Character))
  (bind _s_char_defaultvariables (Variables|/Game/Nibs_Project/Blueprint/Player_Character/Nibs/BP_NibbsCharacter.BP_NibbsCharacter_C|GetS_Char_DefaultVariables _as_bp_nibs_character))
  (bind (_capsulehalfheightdefault _mesh_loc_default _inputcurve _jogspeeddefault _walkspeeddefault _groundfrictiondefault _brakingdecelwalkdefault _spawnloc _actorrotationdefault _tmap8pointnearoffset) (Utilities|Struct|BreakS_Char_DefaultVariableInfo _s_char_defaultvariables))
  (Utilities|Struct|SetmembersinS_Char_DefaultVariableInfo _s_char_defaultvariables _capsulehalfheightdefault _mesh_loc_default _inputcurve _jogspeeddefault _walkspeeddefault _groundfrictiondefault _brakingdecelwalkdefault SpawnLoc _actorrotationdefault _tmap8pointnearoffset))

(fn FUnloadAllMaps
  (params (Level%20to%20load :type E_LevelList%20Enum :default "NewEnumerator0"))
  (switch Utilities|FlowControl|Switch|SwitchonE_LevelList Level%20to%20load
    (:NewEnumerator3
      (Variables|/Script/Engine.LevelStreaming|SetbShouldBeLoaded (Variables|Default|GetNibbsTownLvl_Inst) false)
      (Variables|/Script/Engine.LevelStreaming|SetbShouldBeLoaded (Variables|Default|GetTutorialLevel_Inst) false)
      (Variables|/Script/Engine.LevelStreaming|SetbShouldBeLoaded (Variables|Default|GetNibbsTownLevel) false)
      (Variables|/Script/Engine.LevelStreaming|SetbShouldBeLoaded (Variables|Default|GetBackroomsLvl_Inst) false)
      (return))
    (:NewEnumerator4
      (Variables|/Script/Engine.LevelStreaming|SetbShouldBeLoaded (Variables|Default|GetTutorialLevel_Inst) false)
      (Variables|/Script/Engine.LevelStreaming|SetbShouldBeLoaded (Variables|Default|GetFloor1Level_Inst) false)
      (Variables|/Script/Engine.LevelStreaming|SetbShouldBeLoaded (Variables|Default|GetBackroomsLvl_Inst) false)
      (return))
    (:NewEnumerator5
      (Variables|/Script/Engine.LevelStreaming|SetbShouldBeLoaded (Variables|Default|GetNibbsTownLvl_Inst) false)
      (Variables|/Script/Engine.LevelStreaming|SetbShouldBeLoaded (Variables|Default|GetNibbsTownLevel) false)
      (Variables|/Script/Engine.LevelStreaming|SetbShouldBeLoaded (Variables|Default|GetFloor1Level_Inst) false)
      (Variables|/Script/Engine.LevelStreaming|SetbShouldBeLoaded (Variables|Default|GetBackroomsLvl_Inst) false)
      (return))
    (:NewEnumerator6
      (Variables|/Script/Engine.LevelStreaming|SetbShouldBeLoaded (Variables|Default|GetNibbsTownLvl_Inst) false)
      (Variables|/Script/Engine.LevelStreaming|SetbShouldBeLoaded (Variables|Default|GetNibbsTownLevel) false)
      (Variables|/Script/Engine.LevelStreaming|SetbShouldBeLoaded (Variables|Default|GetFloor1Level_Inst) false)
      (Variables|/Script/Engine.LevelStreaming|SetbShouldBeLoaded (Variables|Default|GetTutorialLevel_Inst) false)
      (return))))

(fn FRegisterMappingContext
  (bind _returnvalue (Game|GetPlayerController 0))
  (bind _returnvalue_2 (PlayerController|LocalPlayerSubsystems|GetEnhancedInputLocalPlayerSubsystem _returnvalue))
  (bind _returnvalue_3 (Class|EnhancedInputSubsystemInterface|GetUserSettings _returnvalue_2))
  (Utilities|FlowControl|Sequence
    (:then_0
      (if (Class|EnhancedInputUserSettings|IsMappingContextRegistered _returnvalue_3 "/Game/Nibs_Project/Input/NibsInput/IM_NibsController.IM_NibsController")
        (Development|PrintString "Mapping Context already registered")
        (else
          (bind _returnvalue_4 (Class|EnhancedInputUserSettings|RegisterInputMappingContext _returnvalue_3 "/Game/Nibs_Project/Input/NibsInput/IM_NibsController.IM_NibsController"))
          (if (not _returnvalue_4)
            (Development|PrintString "false on register nibs control")))))
    (:then_1
      (if (Class|EnhancedInputUserSettings|IsMappingContextRegistered _returnvalue_3 "/Game/Nibs_Project/Input/MenusInput/IM_MenuNavigation.IM_MenuNavigation")
        (Development|PrintString "Mapping Context already registered")
        (else
          (bind _returnvalue_5 (Class|EnhancedInputUserSettings|RegisterInputMappingContext _returnvalue_3 "/Game/Nibs_Project/Input/MenusInput/IM_MenuNavigation.IM_MenuNavigation"))
          (if (not _returnvalue_5)
            (Development|PrintString "False on register menu navigation")))))
    (:then_2
      (if (Class|EnhancedInputUserSettings|IsMappingContextRegistered _returnvalue_3 "/Game/Nibs_Project/Input/MenusInput/IM_ToggleMenu.IM_ToggleMenu")
        (Development|PrintString "Mapping Context already registered")
        (else
          (bind _returnvalue_6 (Class|EnhancedInputUserSettings|RegisterInputMappingContext _returnvalue_3 "/Game/Nibs_Project/Input/MenusInput/IM_ToggleMenu.IM_ToggleMenu"))
          (if (not _returnvalue_6)
            (Development|PrintString "False on register toggle menu")))))
    (:then_3
      (if (Class|EnhancedInputUserSettings|IsMappingContextRegistered _returnvalue_3 "/Game/Nibs_Project/Input/NibsInput/IM_NibsControllerJoyCombat.IM_NibsControllerJoyCombat")
        (Development|PrintString "Mapping Context already registered")
        (else
          (bind _returnvalue_7 (Class|EnhancedInputUserSettings|RegisterInputMappingContext _returnvalue_3 "/Game/Nibs_Project/Input/NibsInput/IM_NibsControllerJoyCombat.IM_NibsControllerJoyCombat"))
          (if (not _returnvalue_7)
            (Development|PrintString "False on register ControllerCombatJOystick")))))
    (:then_4
      (if (Class|EnhancedInputUserSettings|IsMappingContextRegistered _returnvalue_3 "/Game/Nibs_Project/Input/NibsInput/IM_NibsControllerJoyParkour.IM_NibsControllerJoyParkour")
        (Development|PrintString "Mapping Context already registered")
        (else
          (bind _returnvalue_8 (Class|EnhancedInputUserSettings|RegisterInputMappingContext _returnvalue_3 "/Game/Nibs_Project/Input/NibsInput/IM_NibsControllerJoyParkour.IM_NibsControllerJoyParkour"))
          (if (not _returnvalue_8)
            (Development|PrintString "False on register ControllerParkourJOystick")))))))