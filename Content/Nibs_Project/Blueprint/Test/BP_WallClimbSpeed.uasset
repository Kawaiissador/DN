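; Test actor that measures the Nibs character's wall climb speed between Floor and Ceilling overlap components, printing results on screen.
; Leaving Floor restarts a Timeline as a stopwatch, which prints elapsed time as it updates; entering either component stops it.
; These overlaps also print the character's capsule velocity magnitude and game time, though any actor drives the stopwatch.
; An unconnected branch would log the same for other physics objects.
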(event OnComponentBeginOverlap(Floor)
  (params (OverlappedComponent :type Primitive%20Component%20Object%20Reference) (OtherActor :type Actor%20Object%20Reference) (OtherComp :type Primitive%20Component%20Object%20Reference) (OtherBodyIndex :type Integer) (bFromSweep :type Boolean) (SweepResult :type Hit%20Result%20Structure%20%28by%20ref%29))
  (Utilities|FlowControl|Sequence
    (:then_0
      (bind _asbp_nibs_character (Utilities|Casting|CastToBP_NibsCharacter (stale OnComponentBeginOverlap(Ceilling) OtherActor)))
      (bind _returnvalue (Physics|GetPhysicsLinearVelocity (Variables|/Script/Engine.Character|GetCapsuleComponent _asbp_nibs_character) "None"))
      (Development|PrintString (Utilities|String|ToString(Float) (Math|Vector|VectorLength _returnvalue)) true true "(R=0.000000,G=1.000000,B=0.074043,A=1.000000)" 1e+01)
      (Development|PrintString (Utilities|String|ToString(Float) (Utilities|Time|GetGameTimeinSeconds)) true true "(R=0.000000,G=1.000000,B=0.074043,A=1.000000)" 1e+01)
      (Development|PrintString "Character" true true "(R=0.001084,G=1.000000,B=0.042563,A=1.000000)" 1e+01))
    (:then_1
      (bind _timeelapsed (Timeline|Timeline Stop)
        (:Update
          (Development|PrintString (Utilities|String|ToString(Float) _timeelapsed) true true "(R=0.000000,G=0.000000,B=0.000000,A=1.000000)" 1e+01 "TimeElapsed"))))))

(event OnComponentEndOverlap(Floor)
  (params (OverlappedComponent :type Primitive%20Component%20Object%20Reference) (OtherActor :type Actor%20Object%20Reference) (OtherComp :type Primitive%20Component%20Object%20Reference) (OtherBodyIndex :type Integer))
  (Utilities|FlowControl|Sequence
    (:then_0
      (bind _asbp_nibs_character (Utilities|Casting|CastToBP_NibsCharacter OtherActor))
      (bind _returnvalue (Physics|GetPhysicsLinearVelocity (Variables|/Script/Engine.Character|GetCapsuleComponent _asbp_nibs_character) "None"))
      (Development|PrintString (Utilities|String|ToString(Float) (Math|Vector|VectorLength _returnvalue)) true true "(R=0.000000,G=1.000000,B=0.074043,A=1.000000)" 1e+01)
      (Development|PrintString (Utilities|String|ToString(Float) (Utilities|Time|GetGameTimeinSeconds)) true true "(R=0.000000,G=1.000000,B=0.074043,A=1.000000)" 1e+01)
      (Development|PrintString "Character" true true "(R=0.001084,G=1.000000,B=0.042563,A=1.000000)" 1e+01))
    (:then_1
      (bind _timeelapsed (Timeline|Timeline PlayFromStart)
        (:Update
          (Development|PrintString (Utilities|String|ToString(Float) _timeelapsed) true true "(R=0.000000,G=0.000000,B=0.000000,A=1.000000)" 1e+01 "TimeElapsed"))))))

(event OnComponentBeginOverlap(Ceilling)
  (params (OverlappedComponent :type Primitive%20Component%20Object%20Reference) (OtherActor :type Actor%20Object%20Reference) (OtherComp :type Primitive%20Component%20Object%20Reference) (OtherBodyIndex :type Integer) (bFromSweep :type Boolean) (SweepResult :type Hit%20Result%20Structure%20%28by%20ref%29))
  (Utilities|FlowControl|Sequence
    (:then_0
      (bind _asbp_nibs_character (Utilities|Casting|CastToBP_NibsCharacter OtherActor))
      (bind _returnvalue (Physics|GetPhysicsLinearVelocity (Variables|/Script/Engine.Character|GetCapsuleComponent _asbp_nibs_character) "None"))
      (Development|PrintString (Utilities|String|ToString(Float) (Math|Vector|VectorLength _returnvalue)) true true "(R=0.000000,G=1.000000,B=0.074043,A=1.000000)" 1e+01)
      (Development|PrintString (Utilities|String|ToString(Float) (Utilities|Time|GetGameTimeinSeconds)) true true "(R=0.000000,G=1.000000,B=0.074043,A=1.000000)" 1e+01)
      (Development|PrintString "Character" true true "(R=0.001084,G=1.000000,B=0.042563,A=1.000000)" 1e+01))
    (:then_1
      (bind _timeelapsed (Timeline|Timeline Stop)
        (:Update
          (Development|PrintString (Utilities|String|ToString(Float) _timeelapsed) true true "(R=0.000000,G=0.000000,B=0.000000,A=1.000000)" 1e+01 "TimeElapsed"))))))

(event EventBeginPlay)

(event Collision|EventActorBeginOverlap
  (params (OtherActor :type Actor%20Object%20Reference)))

(event EventTick
  (params (DeltaSeconds :type Float%20%28single-precision%29)))

(fn ConstructionScript)