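; BP_TriggerBox_Timer is a trigger volume that starts or stops a speedrun timer when the player pawn overlaps its box.
; The IsEnd flag picks the role: start boxes zero the Timer on PC_Nibs and set it running, end boxes stop it.
; A DoOnce with a one-second delayed reset debounces repeat overlaps.
; Local timer-print and level-selection nodes are left disconnected.
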(event OnComponentBeginOverlap(Box)
  (params (OverlappedComponent :type Primitive%20Component%20Object%20Reference) (OtherActor :type Actor%20Object%20Reference) (OtherComp :type Primitive%20Component%20Object%20Reference) (OtherBodyIndex :type Integer) (bFromSweep :type Boolean) (SweepResult :type Hit%20Result%20Structure%20%28by%20ref%29))
  (if (== OtherActor (Game|Player|GetPlayerPawn 0))
    (bind _aspc_nibs (Utilities|Casting|CastToPC_Nibs (Game|GetPlayerController 0)))
    (Utilities|FlowControl|DoOnce false :!label _label
      (:Completed
        (if (Variables|Default|GetIsEnd?)
          (Variables|/Game/Nibs_Project/PC_Nibs.PC_Nibs_C|SetIstimerRunning? _aspc_nibs false)
          (else
            ;[0.15 0.15 0.15 0.5] Start timer
            (Variables|/Game/Nibs_Project/PC_Nibs.PC_Nibs_C|SetTimer _aspc_nibs 0.0)
            (Variables|/Game/Nibs_Project/PC_Nibs.PC_Nibs_C|SetIstimerRunning? _aspc_nibs true)))
        (Utilities|FlowControl|Delay 1.0)
        (goto _label Reset)))))

(event EventBeginPlay)

(event Collision|EventActorBeginOverlap
  (params (OtherActor :type Actor%20Object%20Reference)))

(fn ConstructionScript)