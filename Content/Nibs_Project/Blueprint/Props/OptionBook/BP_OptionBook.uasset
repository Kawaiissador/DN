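; Options book prop that Escape toggles, swinging it between a stowed spot on the player and a spot in front of the camera.
; A timeline lerps BookPivot from a scaled-down, pawn-relative offset to full size facing the camera, recomputing both transforms each update.
; CanOpen tracks the toggle and IsOpen is set when opening finishes.
; Closing clears both flags, then reverses the timeline after a short delay.
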(event Custom|PressEscape
  (bind _returnvalue (Game|GetPlayerCameraManager 0))
  (bind _returnvalue_2 (Game|Player|GetPlayerPawn 0))
  (bind _returnvalue_3 (Camera|GetCameraLocation _returnvalue))
  (bind _returnvalue_4 (Transformation|GetActorTransform _returnvalue_2))
  (if (not (Variables|Default|GetCanOpen?))
    (Variables|Default|SetCanOpen? true)
    (bind _alpha (Timeline|T_OpenTransition PlayFromStart)
      (:Update
        (Transformation|SetWorldTransform (Variables|Default|GetBookPivot) (Math|Transform|Lerp(Transform) (Math|Transform|MakeTransform (Math|Transform|TransformLocation _returnvalue_4 (Variables|Default|GetBookPivotOffsetLocDefault)) (Math|Transform|TransformRotation _returnvalue_4 (Variables|Default|GetBookPivotOffsetRotDefault)) "0.250000,0.250000,0.250000") (Math|Transform|MakeTransform (+ _returnvalue_3 (* (Math|Vector|Normalize (Math|Vector|GetForwardVector (Camera|GetCameraRotation _returnvalue))) 28.0)) (Math|Rotator|FindLookatRotation (Transformation|GetWorldLocation (Variables|Default|GetBookPivot)) _returnvalue_3)) _alpha) false false))
      (:Finished
        (if (Variables|Default|GetCanOpen?)
          (Variables|Default|SetIsOpen? true)
          (Variables|Default|SetCanOpen? true))))
    (else
      (Variables|Default|SetCanOpen? false)
      (Variables|Default|SetIsOpen? false)
      (Utilities|FlowControl|Delay 0.5)
      (Timeline|T_OpenTransition ReverseFromEnd))))

(event EventBeginPlay
  (Utilities|Casting|CastToABP_Book (Components|SkeletalMesh|GetAnimInstance (Variables|Default|GetSKM_OptionBook))))

(fn ConstructionScript)