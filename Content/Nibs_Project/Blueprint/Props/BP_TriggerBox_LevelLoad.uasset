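; Trigger volume prop that starts a level transition when the player walks into it.
; When the first player's pawn overlaps the Box, it passes its LevelToTrigger enum value to TriggerLevelTranstion on the PC_Nibs player controller, which handles the transition.
; A DoOnce gate that resets after a short delay blocks rapid repeat triggers.
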(event OnComponentBeginOverlap(Box)
  (params (OverlappedComponent :type Primitive%20Component%20Object%20Reference) (OtherActor :type Actor%20Object%20Reference) (OtherComp :type Primitive%20Component%20Object%20Reference) (OtherBodyIndex :type Integer) (bFromSweep :type Boolean) (SweepResult :type Hit%20Result%20Structure%20%28by%20ref%29))
  (if (== OtherActor (Game|Player|GetPlayerPawn 0))
    (bind _aspc_nibs (Utilities|Casting|CastToPC_Nibs (Game|GetPlayerController 0)))
    (Utilities|FlowControl|DoOnce false :!label _label
      (:Completed
        (Default|TriggerLevelTranstion _aspc_nibs (Variables|Default|GetLevel%20To%20trigger))
        (Utilities|FlowControl|Delay 2.0)
        (goto _label Reset)))))

(event EventBeginPlay)

(event Collision|EventActorBeginOverlap
  (params (OtherActor :type Actor%20Object%20Reference)))

(event EventTick
  (params (DeltaSeconds :type Float%20%28single-precision%29)))

(fn ConstructionScript)